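; BP_Ship_primative is a ship actor that shows a floating interaction prompt when the player is nearby.
; Collider overlaps with BP_ThirdPersonCharacter store or clear the player reference and show or hide InteractionText.
; While that reference is valid, Tick rotates the text to face the player's capsule.
; The graph contains only this prompt logic, with no interaction input or ship behavior.
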(event `self.ReceiveTick`
  (params (DeltaSeconds :type "Float (single-precision)"))
  (bind _playercharacterref (`self.PlayerCharacterRef`))
  (bind _interactiontext (`self.InteractionText`))
  (if (`KismetSystemLibrary.IsValid` _playercharacterref)
    (`SceneComponent.K2_SetWorldRotation` _interactiontext (`KismetMathLibrary.FindLookAtRotation` (`SceneComponent.K2_GetComponentLocation` _interactiontext) (`SceneComponent.K2_GetComponentLocation` (`Character.CapsuleComponent` _playercharacterref))) false false)))

(event `self.Collider.OnComponentBeginOverlap`
  (params (OverlappedComponent :type "PrimitiveComponent Object Reference") (OtherActor :type "Actor Object Reference") (OtherComp :type "PrimitiveComponent Object Reference") (OtherBodyIndex :type Integer) (bFromSweep :type Boolean) (SweepResult :type "HitResult Structure (by ref)"))
  (bind _asbp_third_person_character (cast `/Game/ThirdPerson/Blueprints/BP_ThirdPersonCharacter` OtherActor))
  (if (`KismetSystemLibrary.IsValid` _asbp_third_person_character)
    (set `self.PlayerCharacterRef` _asbp_third_person_character)
    (`SceneComponent.SetVisibility` (`self.InteractionText`) true false)))

(event `self.Collider.OnComponentEndOverlap`
  (params (OverlappedComponent :type "PrimitiveComponent Object Reference") (OtherActor :type "Actor Object Reference") (OtherComp :type "PrimitiveComponent Object Reference") (OtherBodyIndex :type Integer))
  (bind _asbp_third_person_character (cast `/Game/ThirdPerson/Blueprints/BP_ThirdPersonCharacter` OtherActor))
  (if (`KismetSystemLibrary.IsValid` _asbp_third_person_character)
    (set `self.PlayerCharacterRef` null)
    (`SceneComponent.SetVisibility` (`self.InteractionText`) false false)))

(fn `UserConstructionScript`)